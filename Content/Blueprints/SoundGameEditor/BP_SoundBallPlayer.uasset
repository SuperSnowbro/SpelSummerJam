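; BP_SoundBallPlayer is the moving playhead of the sound game editor, sweeping along lines of sound keys and activating them.
; On BeginPlay it caches all BPI_SoundKeyInterface actors and computes the line-end X threshold.
; Each Tick it moves along X and messages keys it has reached at its Z height, removing those that return true.
; Past the threshold, it steps back one LineLength and down one LineHeight to the next line.
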(event EventBeginPlay
  (Variables|Default|SetAdjustedThreshold (+ (Variables|Default|GetLineLength) (.x (Transformation|GetActorLocation)) 0.0))
  (bind _outactors (Actor|GetAllActorswithInterface "/Game/Blueprints/SoundGameEditor/BPI_SoundKeyInterface.BPI_SoundKeyInterface_C"))
  (Variables|Default|SetActorList _outactors))

(event EventTick
  (params (DeltaSeconds :type Float%20%28single-precision%29))
  (bind _returnvalue (Transformation|GetActorLocation))
  (bind _returnvalue_2 (Transformation|GetActorLocation))
  (Transformation|AddActorWorldOffset (Math|Vector|MakeVector (* DeltaSeconds (Variables|Default|GetSpeed)) 0.0 0.0) false true)
  (Utilities|FlowControl|Sequence
    (:then_0
      (for (_array_element _array_index) (Variables|Default|GetActorList)
        (if (Math|Boolean|ANDBoolean (<= (.x (Transformation|GetActorLocation _array_element)) (.x _returnvalue_2)) true (Math|Float|NearlyEqual(Float) (.z (Transformation|GetActorLocation _array_element)) (.z _returnvalue_2) 1e-06))
          (bind _unregister (Class|BPISoundKeyInterface|KeyActivate(Message) _array_element))
          (if _unregister
            (Utilities|Array|RemoveIndex (Variables|Default|GetActorList) _array_index)))))
    (:then_1
      (if (> (.x (Transformation|GetActorLocation)) (Variables|Default|GetAdjustedThreshold))
        (Transformation|SetActorLocation (Math|Vector|MakeVector (- (.x _returnvalue) (Variables|Default|GetLineLength)) (.y _returnvalue) (- (.z _returnvalue) (Variables|Default|GetLineHeight))) false false)))))

(fn ConstructionScript)