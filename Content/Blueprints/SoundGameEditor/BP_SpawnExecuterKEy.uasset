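; BP_SpawnExecuterKEy is a sound game key that spawns an entity through the GameManager's EntitySpawner when activated.
; On BeginPlay it shifts back along X by the ExecuterBuildup collection parameter times ball speed, placing it ahead of its original spot.
; If that crosses the line threshold, it wraps by one LineLength in X and one LineHeight up in Z.
; KeyActivate fires ActivateEvent to request the spawn and returns true.
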(event Custom|ActivateEvent
  (Default|SpawnEntity (Variables|/Game/Blueprints/BP_GameManager.BP_GameManager_C|GetEntitySpawner (Variables|Default|GetGameManager))))

(event EventBeginPlay
  (bind _returnvalue (Transformation|GetActorLocation))
  (bind _myball (Variables|Default|GetMyBall))
  (bind _returnvalue_2 (Rendering|Material|GetScalarParameterValue "/Game/Blueprints/SoundGameEditor/MPC_GameplayParams.MPC_GameplayParams" "ExecuterBuildup" :!class /Script/Engine.KismetMaterialLibrary))
  (Transformation|AddActorWorldOffset (Math|Vector|MakeVector (* _returnvalue_2 (Variables|/Game/Blueprints/SoundGameEditor/BP_SoundBallPlayer.BP_SoundBallPlayer_C|GetSpeed (Variables|Default|GetMyBall)) -1.0) 0.0 0.0) false true)
  (if (<= (.x (Transformation|GetActorLocation)) (- (Variables|/Game/Blueprints/SoundGameEditor/BP_SoundBallPlayer.BP_SoundBallPlayer_C|GetAdjustedThreshold _myball) (Variables|/Game/Blueprints/SoundGameEditor/BP_SoundBallPlayer.BP_SoundBallPlayer_C|GetLineLength _myball)))
    (Transformation|SetActorLocation (Math|Vector|MakeVector (+ (.x _returnvalue) (Variables|/Game/Blueprints/SoundGameEditor/BP_SoundBallPlayer.BP_SoundBallPlayer_C|GetLineLength (Variables|Default|GetMyBall))) (.y _returnvalue) (+ (.z _returnvalue) (Variables|/Game/Blueprints/SoundGameEditor/BP_SoundBallPlayer.BP_SoundBallPlayer_C|GetLineHeight (Variables|Default|GetMyBall)))) false true)))

(fn ConstructionScript)

(fn KeyActivate
  (CallFunction|ActivateEvent)
  (return true))