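; VR player pawn that rides in the game's vehicle and touches executer actors with the motion controllers.
; On BeginPlay it snaps to the GameManager's PlayerVehicle anchor, then starts that vehicle's game after a short delay.
; Each trigger calls GetTouched on BP_TestExecuter actors overlapping that hand's collision.
; A DebugNonVR flag lets mouse input rotate the camera for testing without a headset.
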(event EventBeginPlay
  (Transformation|AttachComponentToComponent (Variables|/Game/Blueprints/BP_PlayerVehicle.BP_PlayerVehicle_C|GetAnchor (Variables|/Game/Blueprints/BP_GameManager.BP_GameManager_C|GetPlayerVehicle (Variables|Default|GetGameManager))) "None" "SnapToTarget" "SnapToTarget" "SnapToTarget" false)
  (Utilities|FlowControl|Delay 5.0)
  (Default|BeginGame (Variables|/Game/Blueprints/BP_GameManager.BP_GameManager_C|GetPlayerVehicle (Variables|Default|GetGameManager))))

(event Input|MouseEvents|MouseX
  (params (AxisValue :type Float%20%28single-precision%29))
  (if (Variables|Default|GetDebugNonVR)
    (Transformation|AddRelativeRotation (Variables|Default|GetCamera) (Math|Rotator|MakeRotator 0.0 (stale Input|MouseEvents|MouseY AxisValue) AxisValue) false false)))

(event Input|MouseEvents|MouseY
  (params (AxisValue :type Float%20%28single-precision%29))
  (if (Variables|Default|GetDebugNonVR)
    (Transformation|AddRelativeRotation (Variables|Default|GetCamera) (Math|Rotator|MakeRotator 0.0 AxisValue (stale Input|MouseEvents|MouseX AxisValue)) false false)))

(event Input|KeyboardEvents|MotionControllerLeftTrigger
  (params (Key :type Key%20Structure :default "AnyKey"))
  (:Pressed
    (CallFunction|TouchExecuters (Variables|Default|GetCollisionSX))))

(event Input|KeyboardEvents|MotionControllerRightTrigger
  (params (Key :type Key%20Structure :default "AnyKey"))
  (:Pressed
    (CallFunction|TouchExecuters (Variables|Default|GetCollisionDX))))

(fn ConstructionScript)

(fn TouchExecuters
  (params (ControllerCollision :type Sphere%20Component%20Object%20Reference))
  (for _array_element (Collision|GetOverlappingActors ControllerCollision "/Game/Blueprints/Executers/BP_TestExecuter.BP_TestExecuter_C" :!class /Script/Engine.PrimitiveComponent)
    (bind _asbp_test_executer (Utilities|Casting|CastToBP_TestExecuter _array_element))
    (Default|GetTouched _asbp_test_executer)))