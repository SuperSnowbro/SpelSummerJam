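; Player starship pawn that races along the GameManager's looping spline at steadily increasing speed, rolling around it.
; Tick advances distance and speed, banks the mesh and publishes its location to a material parameter collection.
; Timelines ease speed in at game start and back up after obstacle hits, which also trigger a camera fade.
; PlayerInput maps HMD or mouse input to roll, but it and the StartGame call are unwired.
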(event Custom|BeginGame
  (Variables|Data|SetCanUpdateSpeed true)
  (bind _alpha (Timeline|InterpSpeed Play)
    (:Update
      (Variables|Data|SetCurrentSpeed (Math|Float|Lerp 0.0 (Variables|MechanicsTuning|GetSpeed) _alpha)))))

(event Custom|BadObstacleHitFeedback
  (Variables|Data|SetCanUpdateSpeed false)
  (CameraFades|StartCameraFade (Game|GetPlayerCameraManager 0) (Variables|FeedbackTuning|GetBadObstacleHitFadeAlpha) 0.0 (Variables|FeedbackTuning|GetBadObstacleHitDuration) (Variables|FeedbackTuning|GetBadObstacleHitFeedbackColor) false true)
  (Components|Timeline|SetPlayRate (Variables|Default|GetHitSlowDown) (/ 1.0 (Variables|FeedbackTuning|GetBadObstacleHitDuration)))
  (bind _alpha (Timeline|HitSlowDown PlayFromStart)
    (:Update
      (Variables|Data|SetCurrentSpeed (* (Variables|MechanicsTuning|GetSpeed) (Math|Float|Lerp (Variables|FeedbackTuning|GetHitSlowDownMultiplier) 1.0 _alpha))))
    (:Finished
      (Variables|Data|SetCanUpdateSpeed true))))

(event EventTick
  (params (DeltaSeconds :type Float%20%28single-precision%29))
  (CallFunction|AdvanceAlongSpline)
  (|StarshipFeedback)
  (CallFunction|IncrementSpeed))

(event Input|KeyboardEvents|SpaceBar
  (params (Key :type Key%20Structure :default "AnyKey")))

(fn ConstructionScript)

(fn AdvanceAlongSpline
  (bind _gamemanager (Variables|Setup|GetGameManager))
  (bind _splinesystem (Variables|/Game/Blueprints/BP_GameManager.BP_GameManager_C|GetSplineSystem _gamemanager))
  (bind _spline (Variables|/Game/Blueprints/BP_SPlineSystemSnow.BP_SplineSystemSnow_C|GetSpline _splinesystem))
  (Utilities|FlowControl|Sequence
    (:then_0
      (Variables|Data|SetCurrentDistance (+ (* (Utilities|Time|GetWorldDeltaSeconds) (Variables|Data|GetCurrentSpeed)) (Variables|Data|GetCurrentDistance)))
      (if (> (Variables|Data|GetCurrentDistance) (Spline|GetSplineLength (Variables|/Game/Blueprints/BP_SPlineSystemSnow.BP_SplineSystemSnow_C|GetSpline (Variables|/Game/Blueprints/BP_GameManager.BP_GameManager_C|GetSplineSystem (Variables|Setup|GetGameManager)))))
        (Variables|Data|SetCurrentDistance (- (Variables|Data|GetCurrentDistance) (Spline|GetSplineLength (Variables|/Game/Blueprints/BP_SPlineSystemSnow.BP_SplineSystemSnow_C|GetSpline (Variables|/Game/Blueprints/BP_GameManager.BP_GameManager_C|GetSplineSystem (Variables|Setup|GetGameManager))))))))
    (:then_1
      (Transformation|SetWorldLocationAndRotation (Variables|Default|GetSplinePos) (Spline|GetLocationatDistanceAlongSpline _spline (Variables|Data|GetCurrentDistance) "World") (Math|Rotator|MakeRotator (Variables|Data|GetCurrentRotation) (.pitch (Spline|GetRotationatDistanceAlongSpline _spline (Variables|Data|GetCurrentDistance) "World")) (.yaw (Spline|GetRotationatDistanceAlongSpline _spline (Variables|Data|GetCurrentDistance) "World"))) false true))))

(fn PlayerInput
  (bind _deviceposition (Class|HeadMountedDisplayFunctionLibrary|GetOrientationandPosition))
  (bind _inputremapcurvehmd (Variables|Setup|GetInputRemapCurveHMD))
  (bind _inputsensitivityinvertedhmd (LocalVariables|GetInputSensitivityInvertedHMD))
  (bind _returnvalue (Utilities|IsOutsideFloatInverter (.y _deviceposition)))
  (bind _returnvalue_2 (/ _returnvalue _inputsensitivityinvertedhmd))
  (bind _returnvalue_3 (Math|Float|Clamp(Float) _returnvalue_2 -1.0))
  (bind _returnvalue_4 (Math|Float|Absolute(Float) _returnvalue_3))
  (bind _returnvalue_5 (> _returnvalue_3 0.0))
  (bind _returnvalue_6 (Math|Curves|GetFloatValue _inputremapcurvehmd _returnvalue_4))
  (bind _returnvalue_7 (* _returnvalue_6 -1.0))
  (bind _returnvalue_8 (Math|Float|SelectFloat _returnvalue_6 _returnvalue_7 _returnvalue_5))
  (Utilities|IsHMDSwitch
    (:Has%20HMD
      (Variables|Data|SetCurrentHMDInput _returnvalue_8)
      (Variables|Data|SetCurrentRotation (+ (Variables|Data|GetCurrentRotation) (* _returnvalue_8 (Utilities|Time|GetWorldDeltaSeconds) (Variables|MechanicsTuning|GetTurnRate)))))
    (:No%20HMD
      (Variables|Data|SetCurrentMouseInput (Math|Float|Clamp(Float) (+ (Utilities|IsOutsideFloatInverter (* (Class|Actor|GetInputAxisKeyValue) 1e+01)) (Variables|Data|GetCurrentMouseInput)) -4e+02 4e+02))
      (Variables|Data|SetCurrentRotation (+ (Variables|Data|GetCurrentRotation) (* (Variables|Data|GetCurrentMouseInput) (Utilities|Time|GetWorldDeltaSeconds))))))
  (return))

(fn IncrementSpeed
  (if (Variables|Data|GetCanUpdateSpeed)
    (bind _output_get (Variables|MechanicsTuning|SetSpeed (+ (Variables|MechanicsTuning|GetSpeed) (* (Variables|MechanicsTuning|GetSpeedIncrement) (Utilities|Time|GetWorldDeltaSeconds)))))
    (Variables|Data|SetCurrentSpeed _output_get)))