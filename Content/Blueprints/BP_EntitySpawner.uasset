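; BP_EntitySpawner spawns BP_TestExecuter actors and attaches them to the player vehicle's Anchor via GameManager.
; SpawnEntity uses the given location, or for a zero vector cycles a looping MultiGate through four boxes to pick a random point, then adds Offset.
; GetSpawnPoint samples each box from its relative location and bounds extent.
; IsCloseToAnyPoint tests squared distances against OccupiedSpawnPoints, but nothing here calls it.
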(event Custom|SpawnEntity
  (params (Location :type Vector))
  (Development|PrintString "Spawning" true true "(R=0.000000,G=0.660000,B=1.000000,A=1.000000)" 0.4)
  (if (Math|Vector|Equal(Vector) Location "0,0.000000, 0" 0.0001)
    (Utilities|FlowControl|MultiGate false true -1
      (:Out%200
        (Variables|Default|SetPickedPoint (CallFunction|GetSpawnPoint (Variables|Default|GetSpawnBox))))
      (:Out%201
        (Variables|Default|SetPickedPoint (CallFunction|GetSpawnPoint (Variables|Default|GetBox))))
      (:Out%202
        (Variables|Default|SetPickedPoint (CallFunction|GetSpawnPoint (Variables|Default|GetBox1))))
      (:Out%203
        (Variables|Default|SetPickedPoint (CallFunction|GetSpawnPoint (Variables|Default|GetBox2)))))
    (else
      (Variables|Default|SetPickedPoint Location)))
  (bind _returnvalue (Game|SpawnActorfromClass "/Game/Blueprints/Executers/BP_TestExecuter.BP_TestExecuter_C" (Math|Transform|MakeTransform (+ (Variables|Default|GetPickedPoint) (Variables|Default|GetOffset)) "0, 0, 0" "1,1,1") "Undefined" 0 0))
  (Transformation|AttachComponentToComponent _returnvalue (Variables|/Game/Blueprints/BP_PlayerVehicle.BP_PlayerVehicle_C|GetAnchor (Variables|/Game/Blueprints/BP_GameManager.BP_GameManager_C|GetPlayerVehicle (Variables|Default|GetGameManager))) "None" "KeepRelative" "KeepRelative" "KeepRelative" false))

(fn ConstructionScript)

(fn GetSpawnPoint
  (params (Box :type Box%20Component%20Object%20Reference))
  (return (Math|Random|RandomPointinBoundingBox (Variables|/Script/Engine.SceneComponent|GetRelativeLocation Box) (.BoxExtent (Collision|GetComponentBounds Box)))))

(fn IsClosetoAnyPoint
  (params (PickedPoint :type Vector))
  (for _array_element (Variables|Default|GetOccupiedSpawnPoints)
    (Development|PrintString (Utilities|String|ToString(Float) (Math|Vector|VectorLengthSquared (- _array_element PickedPoint))))
    (bind _output_get (LocalVariables|SetResult (or (<= (Math|Float|Absolute(Float) (Math|Vector|VectorLengthSquared (- _array_element PickedPoint))) (Math|Float|Power (LocalVariables|GetThreshold) 2.0)) (LocalVariables|GetResult))))
    (Development|PrintString (Utilities|String|ToString(Boolean) _output_get)))
  (return (LocalVariables|GetResult)))