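; BP_TestExecuter is a timed touch target that grades how well it is touched by timing.
; On BeginPlay it plays a timeline, paced by the ExecuterBuildup collection parameter, that drives the beat mesh's scale, a dynamic material's intensity and the current score.
; GetTouched sorts that score into max, medium or low touch events, which are empty stubs.
; If the timeline finishes, IgnoredTouch destroys the actor.
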(event Custom|GetTouched
  (if (>= (Variables|Default|GetCurrentScore) 0.66)
    (CallFunction|MaxScoreTouch)
    (elif (>= (Variables|Default|GetCurrentScore) 0.33)
      (CallFunction|MediumScoreTouch)
      (else
        (CallFunction|LowScoreTouch)))))

(event Custom|MediumScoreTouch)

(event Custom|IgnoredTouch
  (Actor|DestroyActor))

(event Custom|LowScoreTouch)

(event Custom|MaxScoreTouch)

(event EventBeginPlay
  (bind _returnvalue (Rendering|Material|CreateDynamicMaterialInstance (Variables|Default|GetBeatMesh) 0 0 :!class /Script/Engine.PrimitiveComponent))
  (Variables|Default|SetBeatMatInstance _returnvalue)
  (bind _returnvalue_2 (Rendering|Material|GetScalarParameterValue "/Game/Blueprints/SoundGameEditor/MPC_GameplayParams.MPC_GameplayParams" "ExecuterBuildup" :!class /Script/Engine.KismetMaterialLibrary))
  (Components|Timeline|SetPlayRate (Variables|Default|GetAnimationTimeline) (/ 1.0 (+ _returnvalue_2 _returnvalue_2)))
  (bind (_direction _scale _score _colorintensity) (Timeline|AnimationTimeline PlayFromStart)
    (:Update
      (Variables|Default|SetCurrentScore _score)
      (Transformation|SetRelativeScale3D (Variables|Default|GetBeatMesh) (Math|Conversions|ToVector(Float) _scale))
      (Rendering|Material|SetScalarParameterValue (Variables|Default|GetBeatMatInstance) "intensity" _colorintensity :!class /Script/Engine.MaterialInstanceDynamic))
    (:Finished
      (CallFunction|IgnoredTouch))))

(fn ConstructionScript)