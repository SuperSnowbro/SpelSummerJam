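; BP_SoundKey is a key actor that plays a configurable sound when activated and flashes the screen in the key's color.
; GetKeyColor derives that color from Pitch by blending red to blue, and the construction script applies it to a dynamic material on the mesh.
; BeginPlay configures the audio component with sound, pitch and volume.
; KeyActivate calls ActivateEvent for a brief camera fade in that color, then plays the audio.
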(event Custom|ActivateEvent
  (CameraFades|StartCameraFade (Game|GetPlayerCameraManager 0) 0.4 0.0 0.1 (CallFunction|GetKeyColor) false false))

(event EventBeginPlay
  (Audio|Components|Audio|SetPitchMultiplier (Variables|Default|GetAudio) (Variables|Default|GetPitch))
  (Audio|Components|Audio|SetVolumeMultiplier (Variables|Default|GetAudio) (Variables|Default|GetVolume) :!class /Script/Engine.AudioComponent)
  (Audio|Components|Audio|SetSound (Variables|Default|GetAudio) (Variables|Default|GetMySound)))

(event Collision|EventActorBeginOverlap
  (params (OtherActor :type Actor%20Object%20Reference)))

(event EventTick
  (params (DeltaSeconds :type Float%20%28single-precision%29)))

(fn ConstructionScript
  (bind _returnvalue (Rendering|Material|CreateDynamicMaterialInstance (Variables|Default|GetStaticMesh) 0 "/Game/Materials/M_SoundKey.M_SoundKey" :!class /Script/Engine.PrimitiveComponent))
  (Rendering|Material|SetVectorParameterValue _returnvalue "color" (CallFunction|GetKeyColor) :!class /Script/Engine.MaterialInstanceDynamic))

(fn GetKeyColor
  (return (Math|Color|Lerp(LinearColor) "(R=1.000000,G=0.000000,B=0.000000,A=1.000000)" "(R=0.000000,G=0.000000,B=1.000000,A=1.000000)" (- (* (Variables|Default|GetPitch) 2.0) 1.6))))

(fn KeyActivate
  (CallFunction|ActivateEvent)
  (Audio|Components|Audio|Play (Variables|Default|GetAudio) 0.0)
  (return true))